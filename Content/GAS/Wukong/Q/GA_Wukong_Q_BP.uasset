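; Wukong's Q gameplay ability: a targeted forward line attack that stuns and damages characters.
; It waits for user-confirmed target data from its target actor and reticle, turns toward the target, commits, then plays the skill montage.
; Montage notifies run a debug-drawn multi line trace from the owner, using a unique-target array to apply both effects once per character per activation.
; Cancelled targeting or a failed commit cancels the ability.
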(event Ability|EventActivateAbility
  (Utilities|Array|Clear (Variables|Default|GetTargetArray))
  (bind _asivcharacter_base (Utilities|Casting|CastToIVCharacterBase (Ability|GetAvatarActorfromActorInfo)))
  (bind _output_get (Variables|Default|SetOwnerCharacter _asivcharacter_base))
  (bind _asivplayer_controller (Utilities|Casting|CastToIVPlayerController (Pawn|GetController _output_get)))
  (Variables|Default|SetOwnerPlayer%20Controller _asivplayer_controller)
  (|WaitTargetData :ConfirmationType "UserConfirmed" :Class "/Game/GAS/Wukong/Q/BP_Wukong_Q_TargetActir.BP_Wukong_Q_TargetActir_C" :MaxRange 1e+03 :TraceProfile "(Name=\"TargetActorGroundLocation\")" :ReticleClass "/Game/GAS/Wukong/Q/BP_Wukong_Q_Reticle.BP_Wukong_Q_Reticle_C"
    (:ValidData
      (|OrentedtoTarget
        (:OnOrentidEndDelegate
          (bind _returnvalue (Ability|CommitAbility))
          (if _returnvalue
            (|PlayMontageandWaitforEvent :MontageToPlay "/Game/Animation/Montage/WuKong_Skill_Q_Montage.WuKong_Skill_Q_Montage"
              (:OnPlayMontageNotifyBegin
                (bind _outhits (Class|KismetSystemLibrary|LineTraceMultiforObjects (Transformation|GetActorLocation (Variables|Default|GetOwnerCharacter)) (+ (Transformation|GetActorLocation (Variables|Default|GetOwnerCharacter)) (* (Transformation|GetActorForwardVector (Variables|Default|GetOwnerCharacter)) "1000.000000,1000.000000,1000.000000")) (Variables|Default|GetObject%20Types) false (Utilities|Array|MakeArray (Variables|Default|GetOwnerCharacter)) "ForDuration" true))
                (for _array_element _outhits
                  (bind _asivcharacter_base_2 (Utilities|Casting|CastToIVCharacterBase (.hitactor _array_element)))
                  (bind _returnvalue_2 (Utilities|Array|AddUnique (Variables|Default|GetTargetArray) _asivcharacter_base_2))
                  (if (!= _returnvalue_2 -1)
                    (GameplayEffects|ApplyGameplayEffectSpecToSelf (Ability|GetAbilitySystemComponent _asivcharacter_base_2) (Ability|MakeOutgoingGameplayEffectSpec "/Game/GAS/Wukong/Q/GE_Wukong_Q_Stun.GE_Wukong_Q_Stun_C"))
                    (GameplayEffects|ApplyGameplayEffectSpecToSelf (Ability|GetAbilitySystemComponent _asivcharacter_base_2) (Ability|MakeOutgoingGameplayEffectSpec "/Game/GAS/Wukong/Q/GE_Wukong_Q_Damage.GE_Wukong_Q_Damage_C"))))))
            (else
              (Ability|CancelAbility :!label _label))))))
    (:Cancelled
      (goto _label))))

(event Ability|EventOnEndAbility
  (params (bWasCancelled :type Boolean))
  (Utilities|Array|Clear (Variables|Default|GetTargetArray)))